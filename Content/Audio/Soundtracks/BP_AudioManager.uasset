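; BP_AudioManager is an actor that controls the soundtrack across two phases of a level.
; On BeginPlay it fades in the first soundtrack.
; The first overlap of its Box trigger starts the second phase, which fades out that track, plays a transition sound effect after a delay, then fades in the second soundtrack.
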(event OnComponentBeginOverlap(Box)
  (params (OverlappedComponent :type Primitive%20Component%20Object%20Reference) (OtherActor :type Actor%20Object%20Reference) (OtherComp :type Primitive%20Component%20Object%20Reference) (OtherBodyIndex :type Integer) (bFromSweep :type Boolean) (SweepResult :type Hit%20Result%20Structure%20%28by%20ref%29))
  (Utilities|FlowControl|DoOnce false
    (:Completed
      (CallFunction|Start2ndPhase))))

(event Custom|Start%202nd%20phase
  (Audio|Components|Audio|FadeOut (Variables|Default|GetSC_Soundtrack) 7.0 0.0 "Linear" :!class /Script/Engine.AudioComponent)
  (Utilities|FlowControl|Delay 8.0)
  (Audio|Components|Audio|Play (Variables|Default|GetSC_SecondPhaseSFX) 0.0)
  (Utilities|FlowControl|Delay 5.0)
  (Audio|Components|Audio|FadeIn (Variables|Default|GetSC_Soundtrack2) 0.0 1.0 0.0 "Linear" :!class /Script/Engine.AudioComponent))

(event Custom|Start%201st%20phase
  (Audio|Components|Audio|FadeIn (Variables|Default|GetSC_Soundtrack) 2.0 1.0 0.0 "Linear" :!class /Script/Engine.AudioComponent))

(event EventBeginPlay
  (CallFunction|Start1stPhase))

(fn ConstructionScript)